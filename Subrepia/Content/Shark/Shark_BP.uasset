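; Shark actor that chases a Target each Tick, moving forward with swept local offsets at a per-frame speed that rises when far away.
; It snaps to face a nearby target and eases its turn with RInterpTo otherwise, playing audio at very close range.
; Hitting anything other than the first-person character sets a flag that makes the next tick point it straight up and move, then resume the chase.
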(event OnComponentHit(Shark)
  (params (HitComponent :type Primitive%20Component%20Object%20Reference) (OtherActor :type Actor%20Object%20Reference) (OtherComp :type Primitive%20Component%20Object%20Reference) (NormalImpulse :type Vector :default "0, 0, 0") (Hit :type Hit%20Result%20Structure%20%28by%20ref%29))
  (Utilities|Casting|CastToFirstPersonCharacter OtherActor
    (:CastFailed
      (Variables|Default|SetHitOb%20ject true))))

(event EventTick
  (params (DeltaSeconds :type Float%20%28single-precision%29))
  (bind _returnvalue (Transformation|GetActorLocation))
  (bind _target (Variables|Default|GetTarget))
  (bind _returnvalue_2 (Transformation|GetActorLocation _target))
  (bind _returnvalue_3 (Math|Rotator|FindLookatRotation _returnvalue _returnvalue_2))
  (bind _returnvalue_4 (Math|Vector|Distance(Vector) _returnvalue _returnvalue_2))
  (if (not (Variables|Default|GetHitOb%20ject))
    (Utilities|FlowControl|Sequence
      (:then_0
        (if (>= _returnvalue_4 9e+03)
          (Variables|Default|SetSharkSpeed 15.0)
          (else
            (Variables|Default|SetSharkSpeed 1e+01))))
      (:then_1
        (Utilities|IsValid _target
          (:Is%20Valid
            (if (<= _returnvalue_4 2e+03)
              (if (<= _returnvalue_4 2e+02)
                (Audio|Components|Audio|Play (Variables|Default|GetAudio) 0.0))
              (Transformation|SetActorRotation _returnvalue_3)
              (else
                (Transformation|SetActorRotation (Math|Interpolation|RInterpTo (Transformation|GetActorRotation) _returnvalue_3 DeltaSeconds 0.754))))
            (Transformation|AddActorLocalOffset (Math|Vector|MakeVector (Variables|Default|GetSharkSpeed) 0.0 0.0) true false)))))
    (else
      (Variables|Default|SetSharkSpeed 15.0)
      (Transformation|SetActorRotation (Math|Rotator|FindLookatRotation (Transformation|GetActorLocation) (+ (Transformation|GetActorLocation) "0, 0,500.000000")))
      (Transformation|AddActorLocalOffset (Math|Vector|MakeVector (Variables|Default|GetSharkSpeed) 0.0 0.0) true false)
      (Variables|Default|SetHitOb%20ject false))))

(fn ConstructionScript)